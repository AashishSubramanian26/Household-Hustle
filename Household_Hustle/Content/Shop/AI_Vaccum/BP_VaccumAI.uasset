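; BP_VaccumAI is an AI robot vacuum pawn that seeks out and sucks up BP_DUST actors.
; It moves to a dust actor three seconds after BeginPlay and again after each dust overlap.
; A per-tick sphere trace at its Cone finds physics-simulating dust, which a timeline lerps toward the Reference component.
; It heads for BP_Dock when BP_3DVac's DirtCount reaches zero, and its Interact function lets it be grabbed.
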(event Custom|Go
  (Utilities|IsValid "/Game/Tasks/Vaccum/BP_DUST.BP_DUST"
    (:Is%20Valid
      (bind _returnvalue (Actor|GetActorOfClass "/Game/Tasks/Vaccum/BP_DUST.BP_DUST_C"))
      (AI|AIMoveTo self "0, 0, 0" _returnvalue 5.0 false))))

(event Custom|MoveTarget
  (bind _vacuumtarget (Variables|Default|GetVacuumTarget))
  (bind _vacuumtarget_2 (Variables|Default|GetVacuumTarget))
  (Utilities|IsValid _vacuumtarget_2
    (:Is%20Valid
      (Physics|SetSimulatePhysics _vacuumtarget_2 false)
      (Components|Timeline|SetPlayRate (Variables|Default|GetMoveTargetT) 0.3)
      (bind _movetrack (Timeline|MoveTargetT PlayFromStart)
        (:Update
          (Variables|Default|SetLocation (Transformation|GetWorldLocation (Variables|Default|GetReference)))
          (Utilities|IsValid _vacuumtarget
            (:Is%20Valid
              (Transformation|SetWorldLocation _vacuumtarget (Math|Vector|Lerp(Vector) (Transformation|GetWorldLocation (Variables|Default|GetVacuumTarget)) (Variables|Default|GetLocation) _movetrack) false false))))
        (:Finished
          (CallFunction|MoveTarget))))))

(event EventBeginPlay
  (Utilities|FlowControl|Delay 3.0)
  (CallFunction|Go))

(event Collision|EventActorBeginOverlap
  (params (OtherActor :type Actor%20Object%20Reference))
  (Utilities|Casting|CastToBP_DUST OtherActor)
  (Utilities|FlowControl|Delay 1.0)
  (CallFunction|Go))

(event EventTick
  (params (DeltaSeconds :type Float%20%28single-precision%29))
  (bind _cone (Variables|Default|GetCone))
  (bind _returnvalue (Transformation|GetWorldLocation _cone))
  (bind _returnvalue_2 (Math|Vector|GetForwardVector _cone))
  (bind _returnvalue_3 (+ _returnvalue_2 _returnvalue))
  (Utilities|FlowControl|Sequence
    (:then_0
      (bind (_outhit _returnvalue_4) (Collision|SphereTraceByChannel _returnvalue_3 _returnvalue_3 5e+01 "TraceTypeQuery1" false 0 "None"))
      (if _returnvalue_4
        (if (Physics|IsSimulatingPhysics (.HitComponent (Collision|BreakHitResult _outhit)) "None")
          (if (Utilities|ClassIsChildOf (Utilities|GetClass (.HitActor (Collision|BreakHitResult _outhit))) "/Game/Tasks/Vaccum/BP_DUST.BP_DUST_C")
            (Variables|Default|SetVacuumTarget (.HitComponent (Collision|BreakHitResult _outhit)))
            (CallFunction|MoveTarget)
            (else
              (Utilities|FlowControl|Delay 0.001 :!label _label)))
          (else
            (goto _label)))
        (else
          (goto _label))))
    (:then_1
      (bind _returnvalue_5 (Actor|GetActorOfClass "/Game/Tasks/Vaccum/BP_3DVac.BP_3DVac_C"))
      (if (== (Variables|/Game/Tasks/Vaccum/BP_3DVac.BP_3DVac_C|GetDirtCount _returnvalue_5) 0)
        (bind _returnvalue_6 (Actor|GetActorOfClass "/Game/Shop/AI_Vaccum/BP_Dock.BP_Dock_C"))
        (AI|AIMoveTo self (Transformation|GetWorldLocation (Variables|/Game/Shop/AI_Vaccum/BP_Dock.BP_Dock_C|GetArrow _returnvalue_6)) 0 5.0 false)))))

(fn ConstructionScript)

(fn Fridge
  (params (FridgeReference :type BP%20Fridge%20Object%20Reference))
  (return false))

(fn Interact
  (params (Target :type Physics%20Handle%20Component%20Object%20Reference) (Component :type Primitive%20Component%20Object%20Reference) (Bone :type Name :default "None") (Location :type Vector :default "0, 0, 0") (Rotation :type Rotator :default "0, 0, 0"))
  (Physics|Components|PhysicsHandle|GrabComponentatLocationwithRotation Target Component Bone Location Rotation)
  (return true true true))

(fn ReleaseObject
  (params (Target :type Physics%20Handle%20Component%20Object%20Reference) (Component :type Primitive%20Component%20Object%20Reference) (Bone :type Name :default "None") (Location :type Vector :default "0, 0, 0") (Rotation :type Rotator :default "0, 0, 0"))
  (return false false false))