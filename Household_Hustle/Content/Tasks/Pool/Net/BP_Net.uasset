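; Pool net tool that the player picks up and dips to clear trash in the pool cleaning task.
; Interact snaps the mesh to a preset rotation and grabs it through the target's grab component call, allowing pickup only.
; Use plays a timeline that tilts the net's roll, gated by IsDipping against retriggering.
; Pool trash that begins overlapping the sphere during a dip is destroyed.
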(event OnComponentBeginOverlap(Sphere)
  (params (OverlappedComponent :type Primitive%20Component%20Object%20Reference) (OtherActor :type Actor%20Object%20Reference) (OtherComp :type Primitive%20Component%20Object%20Reference) (OtherBodyIndex :type Integer) (bFromSweep :type Boolean) (SweepResult :type Hit%20Result%20Structure%20%28by%20ref%29))
  (if (Variables|Default|GetisDipping)
    (bind _asbp_pool_trash (Utilities|Casting|CastToBP_PoolTrash OtherActor))
    (Default|DestroyTrash _asbp_pool_trash)))

(event Custom|Dip%20Net
  (bind _meshroot (Variables|Default|GetMeshRoot))
  (bind _new_rotation (Variables|Default|GetNew%20Rotation))
  (bind _returnvalue (Transformation|GetWorldRotation _meshroot))
  (if (not (Variables|Default|GetisDipping))
    (Variables|Default|SetisDipping true)
    (bind _rotationalpha (Timeline|TL_DipAnimation PlayFromStart)
      (:Update
        (Transformation|SetRelativeRotation _meshroot (Math|Rotator|MakeRotator (Math|Float|Lerp (.roll _new_rotation) (+ (.roll _new_rotation) -3e+01) _rotationalpha) (.pitch _returnvalue) (.yaw _returnvalue)) false false))
      (:Finished
        (Variables|Default|SetisDipping false)))))

(fn ConstructionScript)

(fn Use
  (CallFunction|DipNet))

(fn Fridge
  (params (FridgeReference :type BP%20Fridge%20Object%20Reference))
  (return false))

(fn Interact
  (params (Target :type Physics%20Handle%20Component%20Object%20Reference) (Component :type Primitive%20Component%20Object%20Reference) (Bone :type Name :default "None") (Location :type Vector :default "0, 0, 0") (Rotation :type Rotator :default "0, 0, 0"))
  (Transformation|SetWorldRotation (Variables|Default|GetMeshRoot) (Variables|Default|GetNew%20Rotation) false false)
  (Physics|Components|PhysicsHandle|GrabComponentatLocationwithRotation Target Component Bone Location Rotation)
  (return true false false))

(fn ReleaseObject
  (params (Target :type Physics%20Handle%20Component%20Object%20Reference) (Component :type Primitive%20Component%20Object%20Reference) (Bone :type Name :default "None") (Location :type Vector :default "0, 0, 0") (Rotation :type Rotator :default "0, 0, 0"))
  (return false false false))