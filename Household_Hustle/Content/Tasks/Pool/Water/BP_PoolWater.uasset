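; Pool water actor for the pool-cleaning task, filled with drifting trash that scales with the game day.
; BeginPlay spawns BP_PoolTrash at random points in PoolBox; Tick spins and moves each piece, picking a new random direction at the bounds.
; TrashRemoved drops pieces from the array and marks the DT_Tasks Pool task done in the player's list widget when TrashCount is zero.
; Boolean flags keep Tick updates and removals from overlapping.
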(event Custom|TrashRemoved
  (params (NewParam :type BP%20Pool%20Trash%20Object%20Reference))
  (if (not (Variables|Default|GetupdatingLeaves))
    (Variables|Default|SetremovingTrash true)
    (bind _returnvalue (Utilities|Array|RemoveItem (Variables|Default|GettrashActorArr) NewParam))
    (if _returnvalue
      (Utilities|FlowControl|Sequence
        (:then_0
          (if (== (Variables|Default|GettrashCount) 0)
            (bind _asbp_first_person_character (Utilities|Casting|CastToBP_FirstPersonCharacter (Game|GetPlayerCharacter 0)))
            (bind _returnvalue_2 (Utilities|GetDataTableRow "/Game/Tasks/TaskList/TaskList/DT_Tasks.DT_Tasks" "Pool")
              (:then
                (bind _array_index (Default|GetTaskIndex (Variables|/Game/FirstPerson/Blueprints/BP_FirstPersonCharacter.BP_FirstPersonCharacter_C|GetListWidget _asbp_first_person_character) _returnvalue_2))
                (Default|UpdateTaskUI (Variables|/Game/FirstPerson/Blueprints/BP_FirstPersonCharacter.BP_FirstPersonCharacter_C|GetListWidget _asbp_first_person_character) "Visible" _returnvalue_2 true _array_index)))))
        (:then_1
          (Variables|Default|SetremovingTrash false))))))

(event EventTick
  (params (DeltaSeconds :type Float%20%28single-precision%29))
  (bind _poolbox (Variables|Default|GetpoolBox))
  (bind _returnvalue (Components|Box|GetScaledBoxExtent _poolbox))
  (bind _returnvalue_2 (Transformation|GetWorldLocation _poolbox))
  (if (Math|Boolean|ANDBoolean (Variables|Default|GetleavesLoaded) (not (Variables|Default|GetremovingTrash)) (> (Variables|Default|GettrashCount) 0))
    (Variables|Default|SetupdatingLeaves true)
    (Utilities|FlowControl|Sequence
      (:then_0
        (for _array_element (Variables|Default|GettrashActorArr)
          (bind _asbp_pool_trash (Utilities|Casting|CastToBP_PoolTrash _array_element))
          (Class|Actor|AddActorWorldRotation _asbp_pool_trash "0.000000,0.050000,0.000000")
          (bind _newparam (CallFunction|InBounds (+ _returnvalue_2 _returnvalue) (- _returnvalue_2 _returnvalue) (+ (* (Variables|/Game/Tasks/Pool/Trash/BP_PoolTrash.BP_PoolTrash_C|GetDirection _asbp_pool_trash) 0.25) (Transformation|GetWorldLocation (Variables|/Game/Tasks/Pool/Trash/BP_PoolTrash.BP_PoolTrash_C|GetPaperSprite _asbp_pool_trash)))))
          (if _newparam
            (Transformation|SetActorLocation _asbp_pool_trash (+ (* (Variables|/Game/Tasks/Pool/Trash/BP_PoolTrash.BP_PoolTrash_C|GetDirection _asbp_pool_trash) 0.25) (Transformation|GetWorldLocation (Variables|/Game/Tasks/Pool/Trash/BP_PoolTrash.BP_PoolTrash_C|GetPaperSprite _asbp_pool_trash))) false false)
            (else
              (Variables|/Game/Tasks/Pool/Trash/BP_PoolTrash.BP_PoolTrash_C|SetDirection _asbp_pool_trash (Math|Vector|MakeVector (Math|Random|RandomFloatinRange -1.0 1.0) (Math|Random|RandomFloatinRange -1.0 1.0) 0.0))))))
      (:then_1
        (Variables|Default|SetupdatingLeaves false)))))

(event EventBeginPlay
  (bind _poolbox (Variables|Default|GetpoolBox))
  (bind _returnvalue (Transformation|GetWorldLocation _poolbox))
  (bind _returnvalue_2 (Components|Box|GetScaledBoxExtent _poolbox))
  (bind _returnvalue_3 (Math|Random|RandomPointinBoundingBox (Math|Vector|MakeVector (.x _returnvalue) (.y _returnvalue) (.z _returnvalue)) _returnvalue_2))
  (bind _asgi_info (Utilities|Casting|CastToGI_Info (Game|GetGameInstance)))
  (Variables|Default|SettrashCount (+ (* (Variables|/Script/Household_Hustle.GameInstanceInfo|Getday _asgi_info) 2) 1))
  (for _index (range 0 (- (Variables|Default|GettrashCount) 1))
    (bind _returnvalue_4 (Game|SpawnActorfromClass "/Game/Tasks/Pool/Trash/BP_PoolTrash.BP_PoolTrash_C" (Math|Transform|MakeTransform (Math|Vector|MakeVector (.x _returnvalue_3) (.y _returnvalue_3) (.z _returnvalue)) (Math|Rotator|MakeRotator 0.0 0.0 (Math|Random|RandomFloatinRange 0.0 3.6e+02)) "1.000000,1.000000,1.000000") "Undefined" "MultiplyWithRoot" 0 self (Math|Vector|MakeVector (Math|Random|RandomFloatinRange -1.0 1.0) (Math|Random|RandomFloatinRange -1.0 1.0) 0.0) 0))
    (Utilities|Array|Add (Variables|Default|GettrashActorArr) _returnvalue_4))
  (Variables|Default|SetleavesLoaded true))

(fn ConstructionScript)

(fn InBounds
  (params (UpperBound :type Vector) (LowerBound :type Vector) (InputCoord :type Vector))
  (bind (_x _y) (Math|Vector|BreakVector UpperBound))
  (bind (_x_2 _y_2) (Math|Vector|BreakVector LowerBound))
  (bind (_x_3 _y_3) (Math|Vector|BreakVector InputCoord))
  (return (Math|Boolean|ANDBoolean (<= _x_3 _x) (>= _x_3 _x_2) (<= _y_3 _y) (>= _y_3 _y_2))))