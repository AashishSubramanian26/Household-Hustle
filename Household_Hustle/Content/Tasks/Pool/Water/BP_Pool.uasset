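; Pool cleanup task actor that fills the pool with drifting trash, with more pieces on later days.
; BeginPlay spawns BP_PoolTrash at random points inside PoolBox, scaling the count with GI_Info's Day.
; Tick moves each piece by a fixed per-frame step, re-rolling its direction when it would leave the box's XY bounds.
; CheckTrashCount marks the DT_Tasks "Pool" task done in the player's list widget once TrashCount is zero.
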(event Custom|CheckTrashCount
  (if (== (Variables|Default|GettrashCount) 0)
    (bind _asbp_first_person_character (Utilities|Casting|CastToBP_FirstPersonCharacter (Game|GetPlayerCharacter 0)))
    (bind _returnvalue (Utilities|GetDataTableRow "/Game/Tasks/TaskList/TaskList/DT_Tasks.DT_Tasks" "Pool")
      (:then
        (bind _array_index (Default|GetTaskIndex (Variables|/Game/FirstPerson/Blueprints/BP_FirstPersonCharacter.BP_FirstPersonCharacter_C|GetListWidget _asbp_first_person_character) _returnvalue))
        (Default|UpdateTaskUI (Variables|/Game/FirstPerson/Blueprints/BP_FirstPersonCharacter.BP_FirstPersonCharacter_C|GetListWidget _asbp_first_person_character) "Visible" _returnvalue true _array_index)))))

(event EventTick
  (params (DeltaSeconds :type Float%20%28single-precision%29))
  (bind _poolbox (Variables|Default|GetpoolBox))
  (bind _returnvalue (Components|Box|GetScaledBoxExtent _poolbox))
  (bind _returnvalue_2 (Transformation|GetWorldLocation _poolbox))
  (if (Variables|Default|GetleavesLoaded)
    (for _array_element (Variables|Default|GettrashActorArr)
      (bind _asbp_pool_trash (Utilities|Casting|CastToBP_PoolTrash _array_element))
      (bind _newparam (CallFunction|InBounds (+ _returnvalue_2 _returnvalue) (- _returnvalue_2 _returnvalue) (+ (* (Variables|/Game/Tasks/Pool/Trash/BP_PoolTrash.BP_PoolTrash_C|GetDirection _asbp_pool_trash) "0.500000,0.500000,0.000000") (Transformation|GetWorldLocation (Variables|/Game/Tasks/Pool/Trash/BP_PoolTrash.BP_PoolTrash_C|GetPaperSprite _asbp_pool_trash)))))
      (if _newparam
        (Transformation|SetActorLocation _asbp_pool_trash (+ (* (Variables|/Game/Tasks/Pool/Trash/BP_PoolTrash.BP_PoolTrash_C|GetDirection _asbp_pool_trash) "0.500000,0.500000,0.000000") (Transformation|GetWorldLocation (Variables|/Game/Tasks/Pool/Trash/BP_PoolTrash.BP_PoolTrash_C|GetPaperSprite _asbp_pool_trash))) false false)
        (else
          (Variables|/Game/Tasks/Pool/Trash/BP_PoolTrash.BP_PoolTrash_C|SetDirection _asbp_pool_trash (Math|Vector|MakeVector (Math|Random|RandomFloatinRange -1.0 1.0) (Math|Random|RandomFloatinRange -1.0 1.0) 0.0)))))))

(event EventBeginPlay
  (bind _poolbox (Variables|Default|GetpoolBox))
  (bind _returnvalue (Transformation|GetWorldLocation _poolbox))
  (bind _returnvalue_2 (Components|Box|GetScaledBoxExtent _poolbox))
  (bind _returnvalue_3 (Math|Random|RandomPointinBoundingBox (Math|Vector|MakeVector (.x _returnvalue) (.y _returnvalue) (.z _returnvalue)) _returnvalue_2))
  (bind _asgi_info (Utilities|Casting|CastToGI_Info (Game|GetGameInstance)))
  (Variables|Default|SettrashCount (+ (* (Variables|/Script/Household_Hustle.GameInstanceInfo|Getday _asgi_info) 2) 1))
  (for _index (range 0 (- (Variables|Default|GettrashCount) 1))
    (bind _returnvalue_4 (Game|SpawnActorfromClass "/Game/Tasks/Pool/Trash/BP_PoolTrash.BP_PoolTrash_C" (Math|Transform|MakeTransform (Math|Vector|MakeVector (.x _returnvalue_3) (.y _returnvalue_3) (.z _returnvalue)) (Math|Rotator|MakeRotator 0.0 0.0 (Math|Random|RandomFloatinRange 0.0 3.6e+02)) "1.000000,1.000000,1.000000") "Undefined" "MultiplyWithRoot" 0 self (Math|Vector|MakeVector (Math|Random|RandomFloatinRange -1.0 1.0) (Math|Random|RandomFloatinRange -1.0 1.0) 0.0) 0))
    (Utilities|Array|Add (Variables|Default|GettrashActorArr) _returnvalue_4))
  (Variables|Default|SetleavesLoaded true))

(fn ConstructionScript)

(fn InBounds
  (params (UpperBound :type Vector) (LowerBound :type Vector) (InputCoord :type Vector))
  (bind (_x _y) (Math|Vector|BreakVector UpperBound))
  (bind (_x_2 _y_2) (Math|Vector|BreakVector LowerBound))
  (bind (_x_3 _y_3) (Math|Vector|BreakVector InputCoord))
  (return (Math|Boolean|ANDBoolean (<= _x_3 _x) (>= _x_3 _x_2) (<= _y_3 _y) (>= _y_3 _y_2))))