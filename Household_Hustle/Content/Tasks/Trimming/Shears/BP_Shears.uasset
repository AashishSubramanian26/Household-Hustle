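; BP_Shears is a trimming tool that the player can pick up and use to cut twigs.
; Interact sets the mesh root's rotation, grabs the component through the passed-in target, and allows pickup and rotation but not dragging.
; Use line-traces a short distance forward from the mesh root with the BP_Plant profile and calls CutTwig on any BP_Twig hit.
; Debug print and trace drawing remain, and Niagara effect spawning is disconnected.
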(fn ConstructionScript
  (|CallParentFunction))

(fn Use
  (bind _meshroot (Variables|Default|GetMeshRoot))
  (bind _returnvalue (Transformation|GetWorldTransform _meshroot))
  (Development|PrintString "Snip")
  (bind _outhit (Class|KismetSystemLibrary|LineTraceSinglebyProfile (.location _returnvalue) (+ (.location _returnvalue) (* (Math|Vector|GetForwardVector (.rotation _returnvalue)) "100.000000,100.000000,100.000000")) "BP_Plant" false 0 "ForOneFrame" true))
  (bind _asbp_twig (Utilities|Casting|CastToBP_Twig (.hitactor _outhit)))
  (Default|CutTwig _asbp_twig))

(fn Interact
  (params (Target :type Physics%20Handle%20Component%20Object%20Reference) (Component :type Primitive%20Component%20Object%20Reference) (Bone :type Name :default "None") (Location :type Vector :default "0, 0, 0") (Rotation :type Rotator :default "0, 0, 0"))
  (Transformation|SetWorldRotation (Variables|Default|GetMeshRoot) (Variables|Default|GetNew%20Rotation) false false)
  (Physics|Components|PhysicsHandle|GrabComponentatLocationwithRotation Target Component Bone Location Rotation)
  (return true true false))