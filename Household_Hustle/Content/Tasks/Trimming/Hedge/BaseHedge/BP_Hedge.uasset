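; BP_Hedge is the hedge actor for a trimming task, completed when all its twigs are removed.
; On BeginPlay it spawns a few BP_Twig actors at random offsets around the Cube's bounds origin, counting them and passing itself as OwnerHedge.
; DeleteTwig decrements the count; at zero it looks up the Hedge row in DT_Tasks and marks that task done in the player character's ListWidget.
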(event Custom|DeleteTwig
  (bind _output_get (Variables|Default|SetTwigCount (- (Variables|Default|GetTwigCount) 1)))
  (if (== _output_get 0)
    (bind _asbp_first_person_character (Utilities|Casting|CastToBP_FirstPersonCharacter (Game|GetPlayerCharacter 0)))
    (bind _returnvalue (Utilities|GetDataTableRow "/Game/Tasks/TaskList/TaskList/DT_Tasks.DT_Tasks" "Hedge")
      (:then
        (bind _array_index (Default|GetTaskIndex (Variables|/Game/FirstPerson/Blueprints/BP_FirstPersonCharacter.BP_FirstPersonCharacter_C|GetListWidget _asbp_first_person_character) _returnvalue))
        (Default|UpdateTaskUI (Variables|/Game/FirstPerson/Blueprints/BP_FirstPersonCharacter.BP_FirstPersonCharacter_C|GetListWidget _asbp_first_person_character) "Visible" _returnvalue true _array_index)))))

(event EventBeginPlay
  (for _index (range 0 2)
    (Variables|Default|SetTwigCount (+ (Variables|Default|GetTwigCount) 1))
    (Game|SpawnActorfromClass "/Game/Tasks/Trimming/Hedge/HedgeLeaves/BP_Twig.BP_Twig_C" (Math|Transform|MakeTransform (- (.Origin (Collision|GetComponentBounds (Variables|Default|GetCube))) (Math|Vector|MakeVector (Math|Random|RandomFloatinRange -5e+01 5e+01) (Math|Random|RandomFloatinRange -3e+01 3e+01) (Math|Random|RandomFloatinRange -5e+01 5e+01))) (Math|Rotator|MakeRotator 0.0 0.0 0.0) "1.000000,1.000000,1.000000") "AlwaysSpawn" "MultiplyWithRoot" 0 self 0)))

(fn ConstructionScript)