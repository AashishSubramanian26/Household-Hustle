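; Cuttable twig belonging to a hedge in the trimming task, with its own health and a world-space health bar.
; Each cut spawns a short-lived Niagara effect just below the twig, lowers its health and updates a reused WBP_CleanMeter widget.
; The bar turns toward the player on each update and hides on a timer.
; At zero health the twig notifies its owning BP_Hedge and destroys itself.
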(event Custom|CutTwig
  (bind _in_asset (Variables|Default|GetIn%20Asset))
  (bind _returnvalue (Game|SpawnActorfromClass "/Script/Niagara.NiagaraActor" (Math|Transform|MakeTransform (- (Transformation|GetActorLocation self) "0.000000,0.000000,30.000000") "0, 0, 0" "1.000000,1.000000,1.000000") "Undefined" "MultiplyWithRoot" 0 0))
  (Class|NiagaraComponent|SetAsset (Variables|/Script/Niagara.NiagaraActor|GetNiagaraComponent _returnvalue) _in_asset true)
  (bind _returnvalue_2 (Animation|GetPlayLength _in_asset))
  (Actor|SetLifeSpan _returnvalue _returnvalue_2)
  (bind _output_get (Variables|Default|SetTwigHealth (- (Variables|Default|GetTwigHealth) 1)))
  (CallFunction|UpdateBar)
  (if (== _output_get 0)
    (bind _asbp_hedge (Utilities|Casting|CastToBP_Hedge (Variables|Default|GetOwnerHedge)))
    (Default|DeleteTwig _asbp_hedge)
    (Actor|DestroyActor)))

(event Custom|UpdateBar
  (bind _widget (Variables|Default|GetWidget))
  (Transformation|SetWorldRotation _widget (Math|Rotator|FindLookatRotation (Transformation|GetActorLocation self) (Transformation|GetActorLocation (Game|Player|GetPlayerPawn 0))) false false)
  (Rendering|SetVisibility _widget true false)
  (Utilities|Time|SetTimerbyEvent (delegate Custom|HideBar) 5.0)
  (bind _aswbp_clean_meter (Utilities|Casting|CastToWBP_CleanMeter (UserInterface|GetWidget _widget)))
  (Progress|SetPercent (Variables|/Game/UI/WBP_CleanMeter.WBP_CleanMeter_C|GetWaterBar _aswbp_clean_meter) (/ (Math|Conversions|ToFloat(Integer) (Variables|Default|GetTwigHealth)) 3.0)))

(event Custom|HideBar
  (Rendering|SetVisibility (Variables|Default|GetWidget) false false))

(fn ConstructionScript)