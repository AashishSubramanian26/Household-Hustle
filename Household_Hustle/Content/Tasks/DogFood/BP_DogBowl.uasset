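; BP_DogBowl is the food bowl for the dog-feeding task.
; Each Fill call raises FoodLevel in small increments, and calls made once it is full trigger Filled.
; Filled acts only while the Sphere is hidden: it reveals it, then marks the "Dog" row from DT_Tasks done in the first-person character's ListWidget.
; The Hydrated function and construction script are empty.
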(event Custom|Filled
  (if (not (Rendering|IsVisible (Variables|Default|GetSphere)))
    (Rendering|SetVisibility (Variables|Default|GetSphere) true false)
    (bind _asbp_first_person_character (Utilities|Casting|CastToBP_FirstPersonCharacter (Game|GetPlayerCharacter 0)))
    (bind _returnvalue (Utilities|GetDataTableRow "/Game/Tasks/TaskList/TaskList/DT_Tasks.DT_Tasks" "Dog")
      (:then
        (bind _array_index (Default|GetTaskIndex (Variables|/Game/FirstPerson/Blueprints/BP_FirstPersonCharacter.BP_FirstPersonCharacter_C|GetListWidget _asbp_first_person_character) _returnvalue))
        (Default|UpdateTaskUI (Variables|/Game/FirstPerson/Blueprints/BP_FirstPersonCharacter.BP_FirstPersonCharacter_C|GetListWidget _asbp_first_person_character) "Visible" _returnvalue true _array_index)))))

(event Custom|Fill
  (if (< (Variables|Default|GetFoodLevel) 1e+02)
    (Variables|Default|SetFoodLevel (+ (Variables|Default|GetFoodLevel) 0.1))
    (else
      (CallFunction|Filled))))

(fn ConstructionScript)

(fn Hydrated)