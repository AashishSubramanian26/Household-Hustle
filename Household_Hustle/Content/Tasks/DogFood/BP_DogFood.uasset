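; BP_DogFood is a grabbable, rotatable dog food bag that pours food into a dog bowl when tipped.
; RotationChange checks the bag mesh's pitch against a threshold, toggling the Niagara pour effect and a looping fill timer together.
; While unpaused, the timer traces straight down from the effect and calls Fill on any BP_DogBowl it hits.
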(event Custom|Filling
  (bind _ns_dogfood (Variables|Default|GetNS_DogFood))
  (bind _returnvalue (Transformation|GetWorldLocation _ns_dogfood))
  (bind _outhit (Class|KismetSystemLibrary|LineTraceSinglebyProfile _returnvalue (- _returnvalue "0.000000,0.000000,100.000000") "BP_Plant" false 0 "ForOneFrame" true))
  (bind _asbp_dog_bowl (Utilities|Casting|CastToBP_DogBowl (.hitactor _outhit)))
  (Default|Fill _asbp_dog_bowl))

(event Custom|Upright
  (bind _ns_dogfood (Variables|Default|GetNS_DogFood))
  (if (Components|Activation|IsActive _ns_dogfood)
    (Components|Activation|Deactivate _ns_dogfood)
    (Utilities|Time|PauseTimerbyHandle (Variables|Default|GetDogFoodTimer))))

(event Custom|Tipped
  (bind _ns_dogfood (Variables|Default|GetNS_DogFood))
  (if (not (Components|Activation|IsActive _ns_dogfood))
    (Components|Activation|Activate _ns_dogfood false)
    (Utilities|Time|UnpauseTimerbyHandle (Variables|Default|GetDogFoodTimer))))

(event EventBeginPlay
  (bind _returnvalue (Utilities|Time|SetTimerbyEvent (delegate Custom|Filling) 0.0075 true))
  (bind _output_get (Variables|Default|SetDogFoodTimer _returnvalue))
  (Utilities|Time|PauseTimerbyHandle _output_get))

(event EventRotationChange
  (if (>= (.pitch (Transformation|GetWorldRotation (Variables|Default|GetBagMesh))) 55.0)
    (CallFunction|Tipped)
    (else
      (CallFunction|Upright))))

(fn ConstructionScript)

(fn Fridge
  (params (FridgeReference :type BP%20Fridge%20Object%20Reference))
  (return false))

(fn Interact
  (params (Target :type Physics%20Handle%20Component%20Object%20Reference) (Component :type Primitive%20Component%20Object%20Reference) (Bone :type Name :default "None") (Location :type Vector :default "0, 0, 0") (Rotation :type Rotator :default "0, 0, 0"))
  (Physics|Components|PhysicsHandle|GrabComponentatLocationwithRotation Target Component Bone Location Rotation)
  (return true true))