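; BP_Vaccum is a grabbable vacuum for the "Vacuum" cleaning task.
; On BeginPlay it shuffles candidate locations and spawns a BP_Dirt cluster at the first, using an offset array, counting each piece.
; Each overlap with dirt decrements the count; at zero it marks the DT_Tasks row done in the player's task list widget.
; Interact grabs the component through the passed physics handle, allowing pickup, rotation and dragging.
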(event EventBeginPlay
  (bind _locations (Variables|Default|GetLocations))
  (Variables|Default|SetTaskStatus false)
  (Utilities|Array|Shuffle _locations)
  (for _index (range 0 0)
    (for _array_element (Variables|Default|GetOffset)
      (Math|Integer|IncrementInt (Variables|Default|GetDirtCount)
        (:%20%20
          (Game|SpawnActorfromClass "/Game/Tasks/Vaccum/BP_Dirt.BP_Dirt_C" (Math|Transform|MakeTransform (+ _array_element (Utilities|Array|Get(acopy) _locations _index)) "0, 0, 0" "1.000000,1.000000,1.000000") "Undefined" "MultiplyWithRoot" 0 0))))))

(event Collision|EventActorBeginOverlap
  (params (OtherActor :type Actor%20Object%20Reference))
  (Utilities|Casting|CastToBP_Dirt OtherActor)
  (bind _result (Math|Integer|DecrementInt (Variables|Default|GetDirtCount))
    (:%20%20
      (if (== _result 0)
        (Variables|Default|SetTaskStatus true)
        (bind _asbp_first_person_character (Utilities|Casting|CastToBP_FirstPersonCharacter (Game|GetPlayerCharacter 0)))
        (bind _returnvalue (Utilities|GetDataTableRow "/Game/Tasks/TaskList/TaskList/DT_Tasks.DT_Tasks" "Vacuum")
          (:then
            (bind _array_index (Default|GetTaskIndex (Variables|/Game/FirstPerson/Blueprints/BP_FirstPersonCharacter.BP_FirstPersonCharacter_C|GetListWidget _asbp_first_person_character) _returnvalue))
            (Default|UpdateTaskUI (Variables|/Game/FirstPerson/Blueprints/BP_FirstPersonCharacter.BP_FirstPersonCharacter_C|GetListWidget _asbp_first_person_character) "Visible" _returnvalue (Variables|Default|GetTaskStatus) _array_index)))))))

(event EventTick
  (params (DeltaSeconds :type Float%20%28single-precision%29)))

(fn ConstructionScript)

(fn Fridge
  (params (FridgeReference :type BP%20Fridge%20Object%20Reference))
  (return false))

(fn Interact
  (params (Target :type Physics%20Handle%20Component%20Object%20Reference) (Component :type Primitive%20Component%20Object%20Reference) (Bone :type Name :default "None") (Location :type Vector :default "0, 0, 0") (Rotation :type Rotator :default "0, 0, 0"))
  (Physics|Components|PhysicsHandle|GrabComponentatLocationwithRotation Target Component Bone Location Rotation)
  (return true true true))