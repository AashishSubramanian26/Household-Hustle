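; BP_DUST is a moving dust actor for the vacuum task that destroys itself when a BP_3DVac overlaps it.
; The construction script sets an InterpToMovement path between relative points A and B over a configurable Duration.
; Each pickup decrements the vacuum's DirtCount.
; At zero, it marks the vacuum's task done and updates the player's task list widget using the DT_Tasks "Vacuum" row.
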(event EventBeginPlay)

(event Collision|EventActorBeginOverlap
  (params (OtherActor :type Actor%20Object%20Reference))
  (Utilities|Casting|CastToBP_3DVac OtherActor)
  (Actor|DestroyActor)
  (bind _returnvalue (Actor|GetActorOfClass "/Game/Tasks/Vaccum/BP_3DVac.BP_3DVac_C"))
  (bind _result (Math|Integer|DecrementInt (Variables|/Game/Tasks/Vaccum/BP_3DVac.BP_3DVac_C|GetDirtCount _returnvalue))
    (:%20%20
      (if (== _result 0)
        (Variables|/Game/Tasks/Vaccum/BP_3DVac.BP_3DVac_C|SetTaskStatus _returnvalue true)
        (bind _asbp_first_person_character (Utilities|Casting|CastToBP_FirstPersonCharacter (Game|GetPlayerCharacter 0)))
        (bind _returnvalue_2 (Utilities|GetDataTableRow "/Game/Tasks/TaskList/TaskList/DT_Tasks.DT_Tasks" "Vacuum")
          (:then
            (bind _array_index (Default|GetTaskIndex (Variables|/Game/FirstPerson/Blueprints/BP_FirstPersonCharacter.BP_FirstPersonCharacter_C|GetListWidget _asbp_first_person_character) _returnvalue_2))
            (Default|UpdateTaskUI (Variables|/Game/FirstPerson/Blueprints/BP_FirstPersonCharacter.BP_FirstPersonCharacter_C|GetListWidget _asbp_first_person_character) "Visible" _returnvalue_2 (Variables|/Game/Tasks/Vaccum/BP_3DVac.BP_3DVac_C|GetTaskStatus _returnvalue) _array_index)))))))

(event EventTick
  (params (DeltaSeconds :type Float%20%28single-precision%29)))

(fn ConstructionScript
  (bind _interptomovement (Variables|Default|GetInterpToMovement))
  (Variables|/Script/Engine.InterpToMovementComponent|SetControlPoints _interptomovement (Utilities|Array|MakeArray (Utilities|Struct|MakeInterpControlPoint (Variables|Default|GetA) true) (Utilities|Struct|MakeInterpControlPoint (Variables|Default|GetB) true)))
  (Variables|/Script/Engine.InterpToMovementComponent|SetDuration _interptomovement (Variables|Default|GetDuration)))