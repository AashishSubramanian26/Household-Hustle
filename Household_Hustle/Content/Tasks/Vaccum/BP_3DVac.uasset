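; A grabbable 3D vacuum for a cleanup task that spawns BP_DUST piles at a shuffled location and pulls dust toward itself.
; While the first-person character overlaps it, a sphere trace retries on a short Delay loop to find physics-simulating dust.
; A timeline disables the dust's physics and lerps it to the Reference component, resuming the search once the target is invalid.
; Ending the overlap stops the pull and restores physics.
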(event Custom|Vacuum%20On
  (bind _vaccum (Variables|Default|Getvaccum))
  (bind _returnvalue (Transformation|GetWorldLocation _vaccum))
  (bind _returnvalue_2 (Math|Vector|GetForwardVector _vaccum))
  (bind _returnvalue_3 (+ _returnvalue_2 _returnvalue))
  (if (Variables|Default|GetActivated?)
    (bind (_outhit _returnvalue_4) (Collision|SphereTraceByChannel _returnvalue_3 _returnvalue_3 1e+02 "TraceTypeQuery1" false 0 "None"))
    (if _returnvalue_4
      (if (Physics|IsSimulatingPhysics (.HitComponent (Collision|BreakHitResult _outhit)) "None")
        (if (Utilities|ClassIsChildOf (Utilities|GetClass (.HitActor (Collision|BreakHitResult _outhit))) "/Game/Tasks/Vaccum/BP_DUST.BP_DUST_C")
          (Variables|Default|SetVacuumTarget (.HitComponent (Collision|BreakHitResult _outhit)))
          (CallFunction|MoveTarget)
          (else
            (Utilities|FlowControl|Delay 0.001 :!label _label)
            (CallFunction|Vacuumon)))
        (else
          (goto _label)))
      (else
        (goto _label)))))

(event Custom|MoveTarget
  (bind _vacuumtarget (Variables|Default|GetVacuumTarget))
  (bind _vacuumtarget_2 (Variables|Default|GetVacuumTarget))
  (Utilities|IsValid _vacuumtarget_2
    (:Is%20Valid
      (Physics|SetSimulatePhysics _vacuumtarget_2 false)
      (Components|Timeline|SetPlayRate (Variables|Default|GetMoveTargetT) 0.3)
      (bind _movetrack (Timeline|MoveTargetT PlayFromStart)
        (:Update
          (Variables|Default|SetLocation (Transformation|GetWorldLocation (Variables|Default|GetReference)))
          (Utilities|IsValid _vacuumtarget
            (:Is%20Valid
              (Transformation|SetWorldLocation _vacuumtarget (Math|Vector|Lerp(Vector) (Transformation|GetWorldLocation (Variables|Default|GetVacuumTarget)) (Variables|Default|GetLocation) _movetrack) false false))
            (:Is%20Not%20Valid
              (CallFunction|Vacuumon))))
        (:Finished
          (CallFunction|MoveTarget))))))

(event EventBeginPlay
  (bind _locations (Variables|Default|GetLocations))
  (Variables|Default|SetTaskStatus false)
  (Utilities|Array|Shuffle _locations)
  (for _index (range 0 0)
    (for _array_element (Variables|Default|GetOffset)
      (Math|Integer|IncrementInt (Variables|Default|GetDirtCount)
        (:%20%20
          (Game|SpawnActorfromClass "/Game/Tasks/Vaccum/BP_DUST.BP_DUST_C" (Math|Transform|MakeTransform (+ _array_element (Utilities|Array|Get(acopy) _locations _index)) "0, 0, 0" "1.000000,1.000000,1.000000") "Undefined" "MultiplyWithRoot" 0 "0.000000,0.000000,0.000000" "0.000000,0.000000,0.000000" 0))))))

(event Collision|EventActorBeginOverlap
  (params (OtherActor :type Actor%20Object%20Reference))
  (Utilities|Casting|CastToBP_FirstPersonCharacter OtherActor)
  (Variables|Default|SetActivated? true)
  (CallFunction|Vacuumon))

(event EventTick
  (params (DeltaSeconds :type Float%20%28single-precision%29)))

(event Collision|EventActorEndOverlap
  (params (OtherActor :type Actor%20Object%20Reference))
  (bind _vacuumtarget (Variables|Default|GetVacuumTarget))
  (Utilities|Casting|CastToBP_FirstPersonCharacter OtherActor)
  (Variables|Default|SetActivated? false)
  (Audio|Components|Audio|Stop (Variables|Default|GetMoveTargetT))
  (Utilities|IsValid _vacuumtarget
    (:Is%20Valid
      (Physics|SetSimulatePhysics _vacuumtarget true))))

(fn ConstructionScript)

(fn Fridge
  (params (FridgeReference :type BP%20Fridge%20Object%20Reference))
  (return false))

(fn Interact
  (params (Target :type Physics%20Handle%20Component%20Object%20Reference) (Component :type Primitive%20Component%20Object%20Reference) (Bone :type Name :default "None") (Location :type Vector :default "0, 0, 0") (Rotation :type Rotator :default "0, 0, 0"))
  (Physics|Components|PhysicsHandle|GrabComponentatLocationwithRotation Target Component Bone Location Rotation)
  (return true true true))

(fn ReleaseObject
  (params (Target :type Physics%20Handle%20Component%20Object%20Reference) (Component :type Primitive%20Component%20Object%20Reference) (Bone :type Name :default "None") (Location :type Vector :default "0, 0, 0") (Rotation :type Rotator :default "0, 0, 0"))
  (return false false false))